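; BulletBP is a projectile actor that explodes on contact with any actor other than its owner.
; On overlap it sphere-traces against WorldDynamic objects toward the other actor's location, with persistent debug drawing left on.
; It then destroys itself and spawns the BulletExplosion emitter at the trace's hit location, without checking that the trace hit.
; It applies no damage, and movement is not set up in its graphs.
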(event `self.ReceiveActorBeginOverlap`
  (params (OtherActor :type "Actor Object Reference"))
  (if (not (== OtherActor (`self.GetOwner`)))
    (bind (_outhit _returnvalue) (`KismetSystemLibrary.SphereTraceSingleForObjects` :`Start` (`self.K2_GetActorLocation` self) :`End` (`self.K2_GetActorLocation` OtherActor) :`Radius` 10.0 :`ObjectTypes` (`|MakeArray` "ObjectTypeQuery2" :!type "EObjectTypeQuery Enum") :`DrawDebugType` "Persistent"))
    (`self.K2_DestroyActor`)
    (`GameplayStatics.SpawnEmitterAtLocation` "/Game/StarterContent/Particles/BulletExplosion.BulletExplosion" (`.Location` (`GameplayStatics.BreakHitResult` _outhit)))))

(fn `UserConstructionScript`)
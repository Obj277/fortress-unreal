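; Player controller that drives the player's tank pawn and sends its jump and horizontal movement input to a server through Socket.IO.
; It caches the PlayerBP pawn on BeginPlay, then calls that pawn's jump and move events directly on input.
; Jumps emit "tankJump" only when the pawn can jump.
; Axis input reaches the pawn on every update, but emits "tankMove" with a JSON axis value only when that value changes.
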(event `self.ReceiveBeginPlay`
  (bind _asplayer_bp (cast `/Game/BluePrint/PlayerBP` (`GameplayStatics.GetPlayerPawn` 0)))
  (set `self.MyPawn` _asplayer_bp))

(event `InputAction|Jump`
  (params (Key :type "Key Structure"))
  (:`Pressed`
    (if (`Character.CanJump` (`self.MyPawn`))
      (`SocketIOClientComponent.Emit` (`self.Socket IOClient`) "tankJump" null "/")
      (`/Game/BluePrint/PlayerBP.OnJump_Event` (`self.MyPawn`)))))

(event `InputAxis|Right`
  (params (AxisValue :type "Float (single-precision)"))
  (if (!= (`self.previousAxisValue`) AxisValue)
    (switch `/Game/BluePrint/TankState` (`/Game/BluePrint/PlayerBP.TankState` (`self.MyPawn`))
      (:`NewEnumerator0`
        _)
      (:`NewEnumerator1`
        _)
      (:`NewEnumerator2`
        _))
    (bind _returnvalue (`SIOJsonObject.ConstructJsonObject`))
    (`SIOJsonObject.SetNumberField` _returnvalue "axisValue" AxisValue)
    (`SocketIOClientComponent.Emit` (`self.Socket IOClient`) "tankMove" (`SIOJLibrary.Conv_JsonObjectToJsonValue` _returnvalue) "/"))
  (`/Game/BluePrint/PlayerBP.OnMove_Event` (`self.MyPawn`) AxisValue)
  (set `self.previousAxisValue` AxisValue))

(fn `UserConstructionScript`)
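; Paper2D player character for a side-view tank that moves along X, jumps with a dust particle, fires bullets and stores health.
; Move, jump, fire and damage events drive it, with sprite flipping for direction and a delay-based fire cooldown.
; Each Tick applies movement, then a TankState machine prioritizes firing, jumping, moving and idle to select the flipbook.
; FireBullet spawns BulletBP ahead of the sprite and starts a timer that clears Fired.
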(event `OnMove_Event`
  (params (`Axis Value` :type "Float (double-precision)"))
  (bind _sprite (`self.Sprite`))
  (bind _sprite_2 (`self.Sprite`))
  ;[1 1 1] Movement Control
  (bind _output_get (set `self.AxisValue` `Axis Value`))
  (bind _returnvalue (`KismetMathLibrary.FTrunc` _output_get))
  (switch `int` _returnvalue
    (:`-1`
      (`SceneComponent.K2_SetRelativeRotation` _sprite_2 (struct :`Yaw` 180.0) false false)
      (`SceneComponent.K2_SetRelativeLocation` _sprite (60.0 0.0 0.0) false false))
    (:`1`
      (`SceneComponent.K2_SetRelativeRotation` :`self` _sprite_2)
      (`SceneComponent.K2_SetRelativeLocation` _sprite (-60.0 0.0 0.0) false false)))
  (set `self.direction` _returnvalue))

(event `OnJump_Event`
  ;[1 1 1] Jumping
  (`GameplayStatics.SpawnEmitterAtLocation` "/Game/Art/Particles/particle_Dust.particle_Dust" (`SceneComponent.K2_GetComponentLocation` (`self.DustBox`)))
  (`self.Jump`))

(event `OnFire_Event`
  ;[1 1 1] Firing
  (if (`self.CanFire`)
    (set `self.CanFire` false)
    (`self.Fire Bullet`)
    (`KismetSystemLibrary.Delay` 1.0)
    (set `self.CanFire` true)))

(event `OnDamaged_Event`
  (params (NextHP :type Integer))
  ;[1 1 1] Damaged
  (set `self.Health` NextHP))

(event `self.ReceiveTick`
  (params (DeltaSeconds :type "Float (single-precision)"))
  ;[1 1 1] Animation State
  (`self.AddMovementInput` (1.0 0.0 0.0) (`self.AxisValue`))
  (bind _isstatechanged (`self.Animate State Machine`))
  (if _isstatechanged
    (`self.Update Paper Flipbook`)))

(fn `Animate State Machine`
  (returns (isStateChanged :type Boolean))
  (switch `/Game/BluePrint/TankState` (`self.TankState`)
    (:`NewEnumerator0`
      _)
    (:`NewEnumerator1`
      _)
    (:`NewEnumerator2`
      _)
    (:`NewEnumerator3`
      _))
  (if (`self.Fired`)
    (if (`|EnumEquality` (`self.TankState`) "NewEnumerator3")
      (return false)
      (else
        (set `self.TankState` "NewEnumerator3")
        (return true)))
    (else
      (switch `/Game/BluePrint/TankState` (`self.TankState`)
        (:`NewEnumerator0`
          _)
        (:`NewEnumerator1`
          _)
        (:`NewEnumerator2`
          _)
        (:`NewEnumerator3`
          _))
      (if (`self.IsJumping`)
        (if (`|EnumEquality` (`self.TankState`) "NewEnumerator2")
          (return false)
          (else
            (set `self.TankState` "NewEnumerator2")
            (return true)))
        (else
          (switch `/Game/BluePrint/TankState` (`self.TankState`)
            (:`NewEnumerator0`
              _)
            (:`NewEnumerator1`
              _)
            (:`NewEnumerator2`
              _)
            (:`NewEnumerator3`
              _))
          (if (`self.Is Moving`)
            (set `self.TankState` "NewEnumerator1")
            (return true)
            (else
              (set `self.TankState` "NewEnumerator0")
              (return true))))))))

(fn `Fire Bullet`
  (bind _returnvalue (`SceneComponent.K2_GetComponentRotation` (`self.Sprite`)))
  (`KismetSystemLibrary.K2_SetTimer` null "OnFireFinished" 0.8)
  (`|SpawnActorFromClass` "/Game/BluePrint/BulletBP.BulletBP_C" (`KismetMathLibrary.MakeTransform` (+ (`self.K2_GetActorLocation`) (* (`KismetMathLibrary.GetForwardVector` _returnvalue) 30.0) (* (`KismetMathLibrary.GetUpVector` _returnvalue) 15.0)) _returnvalue (0.5 0.5 0.5)) "Undefined" "OverrideRootScale" self null))

(fn `OnFireFinished`
  (set `self.Fired` false))

(fn `OnRep_TankState`)

(fn `Update Paper Flipbook`
  (`PaperFlipbookComponent.SetFlipbook` (`self.Sprite`) (select `/Game/BluePrint/TankState` (`self.TankState`) :`NewEnumerator0` "/Game/Art/Texture/Idle1.Idle1" :`NewEnumerator1` "/Game/Art/Texture/Running1.Running1" :`NewEnumerator2` "/Game/Art/Texture/Jump1.Jump1" :`NewEnumerator3` "/Game/Art/Texture/Cannon1.Cannon1" :!type "PaperFlipbook Object Reference")))

(fn `UserConstructionScript`
  (set `CharacterMovementComponent.JumpZVelocity` 400.0 (`self.CharacterMovement`))
  (set `self.JumpMaxHoldTime` 0.1))
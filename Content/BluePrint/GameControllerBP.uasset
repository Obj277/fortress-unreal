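; GameControllerBP is the client-side network controller for a multiplayer tank game synced over Socket.IO.
; On BeginPlay it connects under a random "zao" username, shares the socket with PlayerControllerBP and binds server events.
; Spawn events fill a username-to-tank map and possess the local tank; other events replay actions on mapped tanks or remove them.
; Move, fire and damage skip the local name, jump compares against literal "Zao", and Damage emits hits to the server.
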(event `self.ReceiveBeginPlay`
  (bind _socketioclient (`self.SocketIOClient`))
  (set `self.MyName` (`KismetStringLibrary.Concat_StrStr` "zao" (`KismetStringLibrary.Conv_IntToString` (`KismetMathLibrary.RandomInteger` 10000))))
  (`SocketIOClientComponent.Connect` _socketioclient (`SocketIOClientComponent.AddressAndPort` _socketioclient) null null)
  (bind _asplayer_controller_bp (cast `/Game/BluePrint/PlayerControllerBP` (`GameplayStatics.GetPlayerController` 0)))
  (set `/Game/BluePrint/PlayerControllerBP.Socket IOClient` (`self.SocketIOClient`) _asplayer_controller_bp)
  (`SocketIOClientComponent.BindEventToFunction` (`self.SocketIOClient`) "spawn" "OnSpawn" self "/")
  (`SocketIOClientComponent.BindEventToFunction` (`self.SocketIOClient`) "tankMove" "OnMove" self "/")
  (`SocketIOClientComponent.BindEventToFunction` (`self.SocketIOClient`) "tankJump" "OnJump" self "/")
  (`SocketIOClientComponent.BindEventToFunction` (`self.SocketIOClient`) "tankFire" "OnFire" self "/")
  (`SocketIOClientComponent.BindEventToFunction` (`self.SocketIOClient`) "tankDamaged" "OnDamaged" self "/")
  (`SocketIOClientComponent.BindEventToFunction` (`self.SocketIOClient`) "userDisconnect" "OnDisconnect" self "/")
  (`SocketIOClientComponent.Emit` (`self.SocketIOClient`) "username" (`SIOJLibrary.Conv_StringToJsonValue` (`self.MyName`)) "/"))

(fn `Damage`
  (params (DamagedTank :type "/Game/BluePrint/PlayerBP Object Reference"))
  (bind _username (`self.GetUsername` DamagedTank))
  (bind _returnvalue (`SIOJsonObject.ConstructJsonObject`))
  (`SIOJsonObject.SetStringField` _returnvalue "username" _username)
  (`SocketIOClientComponent.Emit` (`self.SocketIOClient`) "tankDamaged" (`SIOJLibrary.Conv_JsonObjectToJsonValue` _returnvalue) "/")
  (`/Game/BluePrint/PlayerBP.OnDamaged_Event` DamagedTank 0))

(fn `GetUsername`
  (params (Tank :type "/Game/BluePrint/PlayerBP Object Reference"))
  (returns (Username :type String))
  (bind _tanks (`self.Tanks`))
  (bind _values (`BlueprintMapLibrary.Map_Values` _tanks))
  (bind _keys (`BlueprintMapLibrary.Map_Keys` _tanks))
  (return (`|GetArrayItem` _keys (`KismetArrayLibrary.Array_Find` _values Tank))))

(fn `OnDamaged`
  (params (Message :type "SIOJsonValue Object Reference"))
  (bind _returnvalue (`SIOJsonValue.AsObject` Message))
  (bind _returnvalue_2 (`SIOJsonObject.GetStringField` _returnvalue "username"))
  (if (`KismetStringLibrary.NotEqual_StrStr` _returnvalue_2 (`self.MyName`))
    (bind (_value _returnvalue_3) (`BlueprintMapLibrary.Map_Find` (`self.Tanks`) _returnvalue_2))
    (if _returnvalue_3
      (bind _returnvalue_4 (`KismetMathLibrary.FTrunc` (`SIOJsonObject.GetNumberField` _returnvalue "hp")))
      (`/Game/BluePrint/PlayerBP.OnDamaged_Event` _value _returnvalue_4)
      (if (<= _returnvalue_4 0)
        (`self.K2_DestroyActor` (`Pawn.GetController` _value))
        (`self.K2_DestroyActor` _value))
      (else
        (`KismetSystemLibrary.PrintString` "Unknown Player")))))

(fn `OnDisconnect`
  (params (Message :type "SIOJsonValue Object Reference"))
  (bind _tanks (`self.Tanks`))
  (bind _returnvalue (`SIOJsonValue.AsObject` Message))
  (bind _returnvalue_2 (`SIOJsonObject.GetStringField` _returnvalue "username"))
  (bind (_value _returnvalue_3) (`BlueprintMapLibrary.Map_Find` _tanks _returnvalue_2))
  (if _returnvalue_3
    (if (`KismetSystemLibrary.IsValid` _value)
      (`self.K2_DestroyActor` (`Pawn.GetController` _value))
      (`self.K2_DestroyActor` _value)
      (`BlueprintMapLibrary.Map_Remove` _tanks _returnvalue_2)
      (`KismetSystemLibrary.PrintString` "disconnected" true true (struct :`G` 0.66 :`B` 1.0 :`A` 1.0) 4.0))))

(fn `OnFire`
  (params (Message :type "SIOJsonValue Object Reference"))
  (bind _returnvalue (`SIOJsonValue.AsObject` Message))
  (bind _returnvalue_2 (`SIOJsonObject.GetStringField` _returnvalue "username"))
  (if (`KismetStringLibrary.NotEqual_StrStr` _returnvalue_2 (`self.MyName`))
    (bind (_value _returnvalue_3) (`BlueprintMapLibrary.Map_Find` (`self.Tanks`) _returnvalue_2))
    (if _returnvalue_3
      (`/Game/BluePrint/PlayerBP.OnFire_Event` _value)
      (else
        (`KismetSystemLibrary.PrintString` "Unknown Player")))))

(fn `OnJump`
  (params (message :type "SIOJsonValue Object Reference"))
  (bind _returnvalue (`SIOJsonValue.AsObject` message))
  (if (`KismetStringLibrary.NotEqual_StrStr` (`self.MyName`) "Zao")
    (bind (_value _returnvalue_2) (`BlueprintMapLibrary.Map_Find` (`self.Tanks`) (`SIOJsonObject.GetStringField` _returnvalue "username")))
    (if _returnvalue_2
      (bind _returnvalue_3 (`SIOJsonObject.GetObjectField` _returnvalue "location"))
      (`self.K2_SetActorTransform` _value (`KismetMathLibrary.MakeTransform` (`KismetMathLibrary.MakeVector` (`SIOJsonObject.GetNumberField` _returnvalue_3 "x") 0.0 (`SIOJsonObject.GetNumberField` _returnvalue_3 "z"))) false false)
      (`/Game/BluePrint/PlayerBP.OnJump_Event` _value)
      (else
        (`KismetSystemLibrary.PrintString` "Unknown Player")))))

(fn `OnMove`
  (params (message :type "SIOJsonValue Object Reference"))
  (bind _returnvalue (`SIOJsonValue.AsObject` message))
  (bind _returnvalue_2 (`SIOJsonObject.GetStringField` _returnvalue "username"))
  (if (`KismetStringLibrary.NotEqual_StrStr` (`self.MyName`) _returnvalue_2)
    (bind (_value _returnvalue_3) (`BlueprintMapLibrary.Map_Find` (`self.Tanks`) _returnvalue_2))
    (if _returnvalue_3
      (bind _returnvalue_4 (`SIOJsonObject.GetObjectField` _returnvalue "location"))
      (`self.K2_SetActorTransform` _value (`KismetMathLibrary.MakeTransform` (`KismetMathLibrary.MakeVector` (`SIOJsonObject.GetNumberField` _returnvalue_4 "x") 0.0 (`SIOJsonObject.GetNumberField` _returnvalue_4 "z"))) false false)
      (`/Game/BluePrint/PlayerBP.OnMove_Event` _value (`SIOJsonObject.GetNumberField` _returnvalue "axisValue"))
      (else
        (`KismetSystemLibrary.PrintString` "Unknown Player")))))

(fn `OnSpawn`
  (params (Message :type "SIOJsonValue Object Reference"))
  (bind _returnvalue (`GameplayStatics.GetPlayerController` 0))
  (bind _returnvalue_2 (`SIOJsonValue.AsObject` Message))
  (`KismetSystemLibrary.PrintString` (`SIOJLibrary.Conv_JsonObjectToString` _returnvalue_2) true true (struct :`G` 0.66 :`B` 1.0 :`A` 1.0) 60.0)
  (bind _returnvalue_3 (`|SpawnActorFromClass` "/Game/BluePrint/PlayerBP.PlayerBP_C" (`KismetMathLibrary.MakeTransform` (`KismetMathLibrary.MakeVector` (`SIOJsonObject.GetNumberField` (`SIOJsonObject.GetObjectField` _returnvalue_2 "location") "x") 0.0 -1600.0)) "Undefined" "OverrideRootScale" null null))
  (bind _returnvalue_4 (`SIOJsonObject.GetStringField` _returnvalue_2 "username"))
  (`BlueprintMapLibrary.Map_Add` (`self.Tanks`) _returnvalue_4 _returnvalue_3)
  (if (`KismetStringLibrary.EqualEqual_StrStr` (`self.MyName`) _returnvalue_4)
    (`Controller.Possess` _returnvalue _returnvalue_3)
    (bind _asplayer_controller_bp (cast `/Game/BluePrint/PlayerControllerBP` _returnvalue))
    (bind _output_get (set `/Game/BluePrint/PlayerControllerBP.PlayerBP` _returnvalue_3 _asplayer_controller_bp))
    (set `/Game/BluePrint/PlayerBP.Health` (`KismetMathLibrary.FTrunc` (`SIOJsonObject.GetNumberField` _returnvalue_2 "hp")) _output_get)
    (else
      (`Pawn.SpawnDefaultController` _returnvalue_3))))

(fn `UserConstructionScript`)